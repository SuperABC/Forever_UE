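; Terrain actor that builds a block-based terrain from grid data using a single Instanced Static Mesh component.
; UpdateTerrain loops over an X/Y cell range and queries LookupTerrain, defined outside this graph, for each cell's type and height.
; Each cell with a non-empty type adds a scaled world-space instance, offset vertically by height, without clearing existing instances.
; The event graph and construction script are empty.
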(fn `UpdateTerrain`
  (params (x1 :type Integer) (y1 :type Integer) (x2 :type Integer) (y2 :type Integer))
  (for _index (range x1 (+ x2 1))
    (for _index_2 (range y1 (+ y2 1))
      (bind (_type _height) (`self.LookupTerrain` _index _index_2))
      (if (`KismetStringLibrary.NotEqual_StrStr` _type)
        (`InstancedStaticMeshComponent.AddInstance` (`self.InstancedStaticMesh`) (`KismetMathLibrary.MakeTransform` (`KismetMathLibrary.MakeVector` (`KismetMathLibrary.Conv_IntToDouble` (* _index 1000)) (`KismetMathLibrary.Conv_IntToDouble` (* _index_2 1000)) (+ (* _height 100.0) -500.0)) (struct) (10.0 10.0 10.0)) true)))))

(fn `UserConstructionScript`)