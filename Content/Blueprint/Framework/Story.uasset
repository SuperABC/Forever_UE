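; Story actor that drives the dialog UI, showing spoken lines and branching choices.
; BeginPlay creates the MeetOption widget and hands it to the MainController; the first Tick calls GameStart once, deferring the story until after setup.
; UpdateDialog and UpdateDialogBranch spawn SectionSpeaking or SectionOption widgets that reference this actor, collapse MeetOption and switch to UI-only input with a visible cursor.
; Lines with a speaker are formatted as a quote prefixed by the name.
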(event `self.ReceiveBeginPlay`
  (bind _returnvalue (`GameplayStatics.GetPlayerController` 0))
  (set `self.Started` false)
  (bind _returnvalue_2 (`|CreateWidget` "/Game/Blueprint/UI/MeetOption.MeetOption_C" _returnvalue))
  (set `self.MeetOption` _returnvalue_2)
  (set `/Game/Blueprint/UI/MeetOption.StoryActor` self _returnvalue_2)
  (`UserWidget.AddToViewport` _returnvalue_2 0)
  (bind _asplayer_controller (cast `/Game/Blueprint/Player/MainController` _returnvalue))
  (set `/Game/Blueprint/Player/MainController.MeetOption` _returnvalue_2 _asplayer_controller))

(event `self.ReceiveTick`
  (params (DeltaSeconds :type "Float (single-precision)"))
  (if (not (`self.Started`))
    (`self.GameStart`)
    (set `self.Started` true)))

(fn `UpdateDialog`
  (params (speaker :type String) (content :type String))
  (bind _returnvalue (`GameplayStatics.GetPlayerController` 0))
  (bind _returnvalue_2 (`|CreateWidget` "/Game/Blueprint/UI/SectionSpeaking.SectionSpeaking_C" (`GameplayStatics.GetPlayerController` 0)))
  (set `/Game/Blueprint/UI/SectionSpeaking.StoryActor` self _returnvalue_2)
  (`/Game/Blueprint/UI/SectionSpeaking.SetText` _returnvalue_2 (`KismetTextLibrary.Conv_StringToText` (`KismetMathLibrary.SelectString` content (`KismetStringLibrary.Concat_StrStr` speaker ":\"" content "\"") (== (`KismetStringLibrary.Len` speaker) 0))))
  (`Widget.SetVisibility` (`self.MeetOption`) "Collapsed")
  (`UserWidget.AddToViewport` _returnvalue_2 0)
  (`WidgetBlueprintLibrary.SetInputMode_UIOnlyEx` _returnvalue _returnvalue_2)
  (set `PlayerController.bShowMouseCursor` true _returnvalue))

(fn `UpdateDialogBranch`
  (params (options :type "Array of String (by ref)"))
  (bind _returnvalue (`GameplayStatics.GetPlayerController` 0))
  (bind _returnvalue_2 (`|CreateWidget` "/Game/Blueprint/UI/SectionOption.SectionOption_C" (`GameplayStatics.GetPlayerController` 0)))
  (set `/Game/Blueprint/UI/SectionOption.StoryActor` self _returnvalue_2)
  (`/Game/Blueprint/UI/SectionOption.SetOptions` _returnvalue_2 options)
  (`Widget.SetVisibility` (`self.MeetOption`) "Collapsed")
  (`UserWidget.AddToViewport` _returnvalue_2 0)
  (`WidgetBlueprintLibrary.SetInputMode_UIOnlyEx` _returnvalue _returnvalue_2)
  (set `PlayerController.bShowMouseCursor` true _returnvalue))

(fn `UserConstructionScript`)