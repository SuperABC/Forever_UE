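; Populace spawns and destroys the game's named CharacterElement actors from lists of additions and removals.
; UpdatePopulace places each addition at its scaled position with a height offset, gives it a default controller and links it to the Story actor.
; Each head gets a dynamic HeadCube material, with its avatar texture loaded at runtime from a name-built asset path.
; Actors are registered by name through AddInstance, and RemoveInstance returns those to destroy.
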(fn `UpdatePopulace`
  (params (adds :type "Array of Person Structure (by ref)") (removes :type "Array of String (by ref)"))
  (for _array_element adds
    (bind _returnvalue (`|SpawnActorFromClass` "/Game/Blueprint/Element/CharacterElement.CharacterElement_C" (`KismetMathLibrary.MakeTransform` (+ (* (`.pos` (break `Person` _array_element)) 1000.0) (0.0 0.0 200.0))) "AdjustIfPossibleButAlwaysSpawn" "MultiplyWithRoot" null null))
    (bind _returnvalue_2 (`KismetMaterialLibrary.CreateDynamicMaterialInstance` "/Game/Blueprint/Element/HeadCube.HeadCube"))
    (bind _returnvalue_3 (`AssetLoader.LoadAssetFromPath` (`KismetStringLibrary.Concat_StrStr` "/Game/Asset/Textures/Avatars/" (`.avatar` (break `Person` _array_element)) "." (`.avatar` (break `Person` _array_element))) "/Script/Engine.Texture"))
    (`MaterialInstanceDynamic.SetTextureParameterValue` _returnvalue_2 "Avatar" _returnvalue_3)
    (`PrimitiveComponent.SetMaterial` (`/Game/Blueprint/Element/CharacterElement.头部` _returnvalue) 0 _returnvalue_2)
    (bind _returnvalue_4 (`GameplayStatics.GetActorOfClass` "/Game/Blueprint/Framework/Story.Story_C"))
    (set `/Game/Blueprint/Element/CharacterElement.StoryActor` _returnvalue_4 _returnvalue)
    (set `/Game/Blueprint/Element/CharacterElement.Name` (break `Person` _array_element) _returnvalue)
    (`Pawn.SpawnDefaultController` _returnvalue)
    (`self.AddInstance` (break `Person` _array_element) _returnvalue))
  (for _array_element_2 removes
    (bind _instances (`self.RemoveInstance` _array_element_2))
    (`self.K2_DestroyActor` _instances)))

(fn `UserConstructionScript`)