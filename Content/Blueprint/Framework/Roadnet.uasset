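; Roadnet Blueprint that draws a road network as mesh instances on the Roadline component.
; UpdateRoadnet reads segments from GetRoadnet and adds one world-space instance per segment, centred between its endpoints and scaled by length and width.
; Yaw comes from the arccosine of the segment direction against the X axis, signed by a Y-axis check.
; Existing instances are not cleared before adding, and the construction script is empty.
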(fn `UpdateRoadnet`
  (bind _returnvalue (`self.GetRoadnet`))
  (for _array_element _returnvalue
    (bind (_v1 _v2 _width) (break `Connection` _array_element))
    (bind _returnvalue_2 (- _v1 _v2))
    (bind _returnvalue_3 (`KismetMathLibrary.Normal` _returnvalue_2))
    (bind _returnvalue_4 (`KismetMathLibrary.DegAcos` (`KismetMathLibrary.Dot_VectorVector` _returnvalue_3 (1.0 0.0 0.0))))
    (`InstancedStaticMeshComponent.AddInstance` (`self.Roadline`) (`KismetMathLibrary.MakeTransform` (* (+ _v1 _v2) 500.0) (`KismetMathLibrary.MakeRotator` 0.0 0.0 (`KismetMathLibrary.SelectFloat` (* _returnvalue_4 -1.0) _returnvalue_4 (> (`KismetMathLibrary.DegAcos` (`KismetMathLibrary.Dot_VectorVector` _returnvalue_3 (0.0 1.0 0.0))) 90.0))) (`KismetMathLibrary.MakeVector` (* (`KismetMathLibrary.VSize` _returnvalue_2) 10.0) (* _width 10.0) 1.0)) true)))

(fn `UserConstructionScript`)