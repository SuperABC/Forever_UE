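; Terrain Blueprint that adds and removes grid-based surface tiles as instances on TerrainSurface.
; UpdateTerrain looks up each added cell and, if its type is set, places a scaled instance on a fixed grid with height taken from the terrain data.
; New instance indices are stored per cell through SetInstance.
; Removed cells retrieve their indices through RemoveInstance, which are then removed from TerrainSurface.
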(fn `UpdateTerrain`
  (params (adds :type "Array of Coordinate Structure (by ref)") (removes :type "Array of Coordinate Structure (by ref)"))
  (for _array_element adds
    (bind (_x _y) (break `Coordinate` _array_element))
    (bind (_type _height) (`self.LookupTerrain` _x _y))
    (if (`KismetStringLibrary.NotEqual_StrStr` _type)
      (bind _returnvalue (`InstancedStaticMeshComponent.AddInstance` (`self.TerrainSurface`) (`KismetMathLibrary.MakeTransform` (`KismetMathLibrary.MakeVector` (`KismetMathLibrary.Conv_IntToDouble` (* _x 1000)) (`KismetMathLibrary.Conv_IntToDouble` (* _y 1000)) (+ (* _height 100.0) -500.0)) (struct) (10.0 10.0 10.0)) true))
      (`self.SetInstance` _x _y (`|MakeArray` _returnvalue))))
  (for _array_element_2 removes
    (bind (_x_2 _y_2) (break `Coordinate` _array_element_2))
    (bind _ids (`self.RemoveInstance` _x_2 _y_2))
    (`InstancedStaticMeshComponent.RemoveInstances` (`self.TerrainSurface`) _ids)))

(fn `UserConstructionScript`)