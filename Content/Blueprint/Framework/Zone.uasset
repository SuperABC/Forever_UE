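; Zone Blueprint that builds named zone actors in the level from an array of zone data.
; UpdateZone spawns a ZoneElement per entry, scaling center and size into world units and converting rotation from radians to degree yaw.
; Each element receives its name and a reference to this Zone, adds its trigger, sets up its fences, and is registered by name through SetInstance.
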(fn `UpdateZone`
  (params (zones :type "Array of Zone Structure (by ref)"))
  (locals (Fences :type "Array of Fence Structure"))
  (for _array_element zones
    (set `local.Fences` (`.fences` (break `Zone` _array_element)))
    (bind _returnvalue (* (`.center` (break `Zone` _array_element)) 1000.0))
    (bind _returnvalue_2 (`|SpawnActorFromClass` "/Game/Blueprint/Element/ZoneElement.ZoneElement_C" (`KismetMathLibrary.MakeTransform` _returnvalue (`KismetMathLibrary.MakeRotator` 0.0 0.0 (* (/ (`.rotation` (break `Zone` _array_element)) (`KismetMathLibrary.GetPI`)) 180.0))) "AlwaysSpawn" "MultiplyWithRoot" null null))
    (set `/Game/Blueprint/Element/ZoneElement.Center` _returnvalue _returnvalue_2)
    (set `/Game/Blueprint/Element/ZoneElement.Size` (* (`.size` (break `Zone` _array_element)) 10.0) _returnvalue_2)
    (set `/Game/Blueprint/Element/ZoneElement.Name` (break `Zone` _array_element) _returnvalue_2)
    (set `/Game/Blueprint/Element/ZoneElement.Zone` self _returnvalue_2)
    (`/Game/Blueprint/Element/ZoneElement.AddTrigger` _returnvalue_2)
    (`/Game/Blueprint/Element/ZoneElement.SetFences` _returnvalue_2 (`local.Fences`))
    (`self.SetInstance` (break `Zone` _array_element) _returnvalue_2)))

(fn `UserConstructionScript`)