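; Room manages the RoomElement actors that make up named rooms, spawning and removing them on update.
; UpdateRoom spawns one element per added entry, scaling position and size and converting yaw from radians to degrees.
; Each element receives its name, size and owning Room, builds its trigger, then is registered through SetInstance.
; Removed elements are destroyed, and RemoveInstance then clears the given name.
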(fn `UpdateRoom`
  (params (name :type String) (adds :type "Array of Room Structure (by ref)") (removes :type "Array of Actor Object Reference (by ref)"))
  (for _array_element adds
    (bind _returnvalue (`|SpawnActorFromClass` "/Game/Blueprint/Element/RoomElement.RoomElement_C" (`KismetMathLibrary.MakeTransform` (* (`.center` (break `Room` _array_element)) 1000.0) (`KismetMathLibrary.MakeRotator` 0.0 0.0 (* (/ (`.rotation` (break `Room` _array_element)) (`KismetMathLibrary.GetPI`)) 180.0))) "AlwaysSpawn" "MultiplyWithRoot" null null))
    (set `/Game/Blueprint/Element/RoomElement.Center` (0.0 0.0 0.0) _returnvalue)
    (set `/Game/Blueprint/Element/RoomElement.Size` (* (`.size` (break `Room` _array_element)) 10.0) _returnvalue)
    (set `/Game/Blueprint/Element/RoomElement.Name` (break `Room` _array_element) _returnvalue)
    (set `/Game/Blueprint/Element/RoomElement.Room` self _returnvalue)
    (`/Game/Blueprint/Element/RoomElement.AddTrigger` _returnvalue)
    (`self.SetInstance` name _returnvalue))
  (if (not (== (`KismetArrayLibrary.Array_Length` removes) 0))
    (for _array_element_2 removes
      (`self.K2_DestroyActor` _array_element_2))
    (`self.RemoveInstance` name)))

(fn `UserConstructionScript`)