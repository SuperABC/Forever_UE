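; Building blueprint that turns an array of building descriptions into BuildingElement actors in the world.
; UpdateBuilding spawns one element per entry, scaling the center into world units and converting rotation from radians to a yaw in degrees.
; It passes each new element its center, scaled size and walls, then hands it to SetInstance under the entry's name.
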(fn `UpdateBuilding`
  (params (buildings :type "Array of Building Structure (by ref)"))
  (locals (Walls :type "Array of Wall Structure"))
  (for _array_element buildings
    (set `local.Walls` (`.walls` (break `Building` _array_element)))
    (bind _returnvalue (* (`.center` (break `Building` _array_element)) 1000.0))
    (bind _returnvalue_2 (`|SpawnActorFromClass` "/Game/Blueprint/Element/BuildingElement.BuildingElement_C" (`KismetMathLibrary.MakeTransform` _returnvalue (`KismetMathLibrary.MakeRotator` 0.0 0.0 (* (/ (`.rotation` (break `Building` _array_element)) (`KismetMathLibrary.GetPI`)) 180.0))) "AlwaysSpawn" "MultiplyWithRoot" null null))
    (set `/Game/Blueprint/Element/BuildingElement.Center` _returnvalue _returnvalue_2)
    (set `/Game/Blueprint/Element/BuildingElement.Size` (* (`.size` (break `Building` _array_element)) (10.0 10.0 1.0)) _returnvalue_2)
    (`/Game/Blueprint/Element/BuildingElement.SetWalls` _returnvalue_2 (`local.Walls`))
    (`self.SetInstance` (break `Building` _array_element) _returnvalue_2)))

(fn `UserConstructionScript`)