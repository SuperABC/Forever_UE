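; ZoneElement is a Blueprint zone that tells its Zone reference when the player enters or leaves it.
; Collider overlap events filter for player character 0 and pass the element's Name to EnterZone or LeaveZone.
; AddTrigger scales the Collider to Size.
; SetFences stores fence data and adds a cube mesh with the DefaultZone material per fence, converting center and size with fixed multipliers.
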(event `self.Collider.OnComponentBeginOverlap`
  (params (OverlappedComponent :type "PrimitiveComponent Object Reference") (OtherActor :type "Actor Object Reference") (OtherComp :type "PrimitiveComponent Object Reference") (OtherBodyIndex :type Integer) (bFromSweep :type Boolean) (SweepResult :type "HitResult Structure (by ref)"))
  (if (== OtherActor (`GameplayStatics.GetPlayerCharacter` 0))
    (`ZoneBase.EnterZone` (`self.Zone`) (`self.Name`))))

(event `self.Collider.OnComponentEndOverlap`
  (params (OverlappedComponent :type "PrimitiveComponent Object Reference") (OtherActor :type "Actor Object Reference") (OtherComp :type "PrimitiveComponent Object Reference") (OtherBodyIndex :type Integer))
  (if (== (`GameplayStatics.GetPlayerCharacter` 0) OtherActor)
    (`ZoneBase.LeaveZone` (`self.Zone`) (`self.Name`))))

(fn `AddTrigger`
  (`SceneComponent.SetRelativeScale3D` (`self.Collider`) (`self.Size`)))

(fn `SetFences`
  (params (Fences :type "Array of Fence Structure"))
  (bind _output_get (set `self.Fences` Fences))
  (for _array_element _output_get
    (bind _returnvalue (`AddComponent|NODE_AddStaticMeshComponent-1` :`RelativeTransform` (`KismetMathLibrary.MakeTransform` (* (break `Fence` _array_element) 1000.0) (struct) (* (`.size` (break `Fence` _array_element)) 10.0))))
    (`StaticMeshComponent.SetStaticMesh` _returnvalue "/Game/Asset/Meshes/Cube.Cube")
    (`PrimitiveComponent.SetMaterial` _returnvalue 0 "/Game/Asset/Materials/DefaultZone.DefaultZone")))

(fn `UserConstructionScript`)