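; Room element actor that reports when the player character enters or leaves a named room volume.
; Overlap events on its Collider filter for player 0 and call EnterRoom or LeaveRoom on the owning Room reference with this element's name.
; AddTrigger positions and scales the Collider from the stored Center and Size, shrinking it to 99 percent of the size.
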(event `self.Collider.OnComponentBeginOverlap`
  (params (OverlappedComponent :type "PrimitiveComponent Object Reference") (OtherActor :type "Actor Object Reference") (OtherComp :type "PrimitiveComponent Object Reference") (OtherBodyIndex :type Integer) (bFromSweep :type Boolean) (SweepResult :type "HitResult Structure (by ref)"))
  (if (== OtherActor (`GameplayStatics.GetPlayerCharacter` 0))
    (`RoomBase.EnterRoom` (`self.Room`) (`self.Name`))))

(event `self.Collider.OnComponentEndOverlap`
  (params (OverlappedComponent :type "PrimitiveComponent Object Reference") (OtherActor :type "Actor Object Reference") (OtherComp :type "PrimitiveComponent Object Reference") (OtherBodyIndex :type Integer))
  (if (== (`GameplayStatics.GetPlayerCharacter` 0) OtherActor)
    (`RoomBase.LeaveRoom` (`self.Room`) (`self.Name`))))

(fn `AddTrigger`
  (bind _collider (`self.Collider`))
  (`SceneComponent.K2_SetRelativeLocation` _collider (`self.Center`) false false)
  (`SceneComponent.SetRelativeScale3D` _collider (* (`self.Size`) 0.99)))

(fn `UserConstructionScript`)